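; Game Blueprint for Shields N Shaterbolts that runs local multiplayer setup, player-select UI and wizard spawning.
; BeginPlay shows the select widget, caches PlayerStarts and creates local players in a loop.
; Spawning swaps a player's pawn for a wizard at its controller-ID start and lights its card, while despawning swaps in an EmptyPawn, both viewing through CameraActor.
; CheckWin only prints when one wizard remains, and GetRandomSpawn's logic is unwired.
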(event `RemoveUI`
  ;[1 1 1] Remove PlayerSelect UI
  (set `self.InLobby` false)
  (`Widget.RemoveFromParent` (`self.PlayerSelectWidget`)))

(event `self.ReceiveBeginPlay`
  (bind _numberofplayers (`self.NumberOfPlayers`))
  ;[1 1 1] Creates the Players
  (bind _returnvalue (`|CreateWidget` "/Game/UIWidgets/PlayerSelect.PlayerSelect_C"))
  (bind _output_get (set `self.PlayerSelectWidget` _returnvalue))
  (`UserWidget.AddToViewport` _output_get 0)
  (bind _outactors (`GameplayStatics.GetAllActorsOfClass` "/Script/Engine.PlayerStart"))
  (set `self.SpawnPoints` _outactors)
  (while (<= _numberofplayers 3)
    (bind _output_get_2 (set `self.NumberOfPlayers` (+ _numberofplayers 1)))
    (`GameplayStatics.CreatePlayer` _output_get_2)))

(event `SpawnCharacter`
  (params (PlayerController :type "PlayerController Object Reference"))
  (bind _returnvalue (`Controller.K2_GetPawn` PlayerController))
  ;[1 1 1] Spawns Characters
  (`/Engine/EditorBlueprintResources/StandardMacros.IsValid` _returnvalue
    (:`Is Valid`
      (`self.K2_DestroyActor` _returnvalue)
      (bind _aswizard_controller (cast `/Game/Blueprints/WizardController` PlayerController))
      (bind _returnvalue_2 (`GameplayStatics.GetPlayerControllerID` _aswizard_controller))
      (bind _returnvalue_3 (`self.GetTransform` (`|GetArrayItem` (`self.SpawnPoints`) _returnvalue_2)))
      (bind _returnvalue_4 (`|SpawnActorFromClass` "/Game/Blueprints/WizardBP.WizardBP_C" _returnvalue_3 "AdjustIfPossibleButAlwaysSpawn" "OverrideRootScale" null null))
      (`self.ActivatePlayerCard`)
      (set `/Game/Blueprints/WizardBP.SpawnPoint` _returnvalue_3 _returnvalue_4)
      (`Controller.Possess` PlayerController _returnvalue_4)
      (`PlayerController.SetViewTargetWithBlend` PlayerController (`self.CameraActor`) 0.0 "VTBlend_Linear" 0.0 false))))

(event `DespawnCharacter`
  (params (PlayerController :type "PlayerController Object Reference"))
  (bind _returnvalue (`Controller.K2_GetPawn` PlayerController))
  ;[1 1 1] Despawns Characters
  (`/Engine/EditorBlueprintResources/StandardMacros.IsValid` _returnvalue
    (:`Is Valid`
      (`self.K2_DestroyActor` _returnvalue)
      (bind _returnvalue_2 (`|SpawnActorFromClass` "/Game/Blueprints/EmptyPawn.EmptyPawn_C" (`self.GetRandomSpawn`) "AdjustIfPossibleButAlwaysSpawn" "OverrideRootScale" null null))
      (`Controller.Possess` PlayerController _returnvalue_2)
      (`PlayerController.SetViewTargetWithBlend` PlayerController (`self.CameraActor`) 0.0 "VTBlend_Linear" 0.0 false))))

(event `CheckWin`
  ;[1 1 1] Checks for the Win Condition
  (bind _outactors (`GameplayStatics.GetAllActorsOfClass` "/Game/Blueprints/WizardBP.WizardBP_C"))
  (if (== (`KismetArrayLibrary.Array_Length` _outactors) 1)
    (`KismetSystemLibrary.PrintString` "GameFinished")))

(event `ActivatePlayerCard`
  ;[1 1 1] Activate Player Card UI Elements
  (`/Game/UIWidgets/PlayerSelect.ActivateCard` (`self.PlayerSelectWidget`) (stale `SpawnCharacter` _returnvalue_2)))

(fn `UserConstructionScript`)